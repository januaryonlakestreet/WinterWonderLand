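; GM_steam is a Steam session test Blueprint that hosts and searches for sessions through Advanced Sessions nodes on BeginPlay.
; It creates a session tagged with a GAMENAME property, then on success finds and re-filters sessions.
; It reads each result's GAMENAME and compares it to a placeholder string, but the match does nothing.
; The JoinSession node is unwired, so no session is ever joined.
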(event EventBeginPlay
  (bind _returnvalue (Class|AdvancedSessionsLibrary|MakeLiteralSessionSearchProperty :ComparisonOp "Equals"))
  (bind _array (Utilities|Array|MakeArray _returnvalue))
  (|AdvancedSession (Utilities|Array|MakeArray (Class|AdvancedSessionsLibrary|MakeLiteralSessionPropertyString "GAMENAME" "WINTERWONDERLAND")) (Game|GetPlayerController 0) 100 0 false true false true true false false false true ; Make an advanced session with the extra session properties
    (:OnSuccess
      (Development|PrintString "SUCCESS")
      (bind _results (|FindSessionsAdvanced 0 0 false "ClientServersOnly" _array false false false) ; Find Sessions with post filter
        (:OnSuccess
          (bind _filteredresults (Class|FindSessionsCallbackProxyAdvanced|FilterSessionResults _results _array)) ; Stand alone filter - Can be used with the STD Find Sessions
          (bind _array_element (Utilities|Array|ForEachLoopwithBreak _filteredresults)
            (:LoopBody
              (bind _extrasettings (Class|AdvancedSessionsLibrary|GetExtraSettings _array_element))
              (bind _settingvalue (Class|AdvancedSessionsLibrary|GetSessionPropertyString _extrasettings "GAMENAME") ; Check if this session has the property
                (:Found
                  (if (Utilities|Enum|Equal(Enum) _settingvalue "This is your game name")
                    _))))))))
    (:OnFailure
      (Development|PrintString "F"))))

(fn ConstructionScript)